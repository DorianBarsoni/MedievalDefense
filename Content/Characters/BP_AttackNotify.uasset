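; BP_AttackNotify is an animation notify that applies a troop's attack damage when it fires.
; It damages the blackboard's EnemyChased troop using the attacker's data asset, or falls back to the Castle construct when that target is invalid.
; On a kill, it flags the victim dead in its blackboard, removes it from the controller's EnemiesToAttack, then retargets the next enemy or clears the sight and range flags.
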(fn ReceivedNotify
  (params (MeshComp :type Skeletal%20Mesh%20Component%20Object%20Reference) (Animation :type Anim%20Sequence%20Base%20Object%20Reference) (EventReference :type Anim%20Notify%20Event%20Reference%20Structure%20%28by%20ref%29))
  (bind _astroop_character (Utilities|Casting|CastToTroopCharacter (Components|GetOwner MeshComp)))
  (if (Utilities|IsValid (AI|Components|Blackboard|GetValueasObject (AI|GetBlackboard _astroop_character) (Variables|Default|GetEnemyChased)))
    (bind _astroop_character_2 (Utilities|Casting|CastToTroopCharacter (AI|Components|Blackboard|GetValueasObject (AI|GetBlackboard _astroop_character) (Variables|Default|GetEnemyChased))))
    (Class|TroopCharacter|GetDamage _astroop_character_2 (Variables|/Script/MedievalDefense.TroopDataAsset|GetAttackDamage (Variables|/Script/MedievalDefense.TroopCharacter|GetTroopDataAsset _astroop_character)))
    (if (<= (Variables|/Script/MedievalDefense.LifeComponent|GetLife (Variables|/Script/MedievalDefense.TroopCharacter|GetLifeComponent _astroop_character_2)) 0)
      (AI|Components|Blackboard|SetValueasBool (AI|GetBlackboard _astroop_character_2) (Variables|Default|GetIsDead) true)
      (bind _astroop_controller (Utilities|Casting|CastToTroopController (Pawn|GetController _astroop_character)))
      (Utilities|Array|RemoveItem (Variables|/Script/MedievalDefense.TroopController|GetEnemiesToAttack _astroop_controller) _astroop_character_2)
      (if (Utilities|Array|IsNotEmpty (Variables|/Script/MedievalDefense.TroopController|GetEnemiesToAttack _astroop_controller))
        (AI|Components|Blackboard|SetValueasObject (AI|GetBlackboard _astroop_character) (Variables|Default|GetEnemyChased) (Utilities|Array|Get(acopy) (Variables|/Script/MedievalDefense.TroopController|GetEnemiesToAttack _astroop_controller)))
        (else
          (AI|Components|Blackboard|SetValueasObject (AI|GetBlackboard _astroop_character) (Variables|Default|GetEnemyChased) 0)
          (AI|Components|Blackboard|SetValueasBool (AI|GetBlackboard _astroop_character) (Variables|Default|GetIsEnemyOnSight) false)
          (AI|Components|Blackboard|SetValueasBool (AI|GetBlackboard _astroop_character) (Variables|Default|GetIsEnemyInRange) false))))
    (return true)
    (else
      (bind _asconstruct (Utilities|Casting|CastToConstruct (AI|Components|Blackboard|GetValueasObject (AI|GetBlackboard _astroop_character) (Variables|Default|GetCastle)))
        (:then
          (Class|Construct|GetDamage _asconstruct (Variables|/Script/MedievalDefense.TroopDataAsset|GetAttackDamage (Variables|/Script/MedievalDefense.TroopCharacter|GetTroopDataAsset _astroop_character)))
          (return true))
        (:CastFailed
          (Development|PrintString "echec"))))))