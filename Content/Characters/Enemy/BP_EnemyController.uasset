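; BP_EnemyController is an enemy AI controller that runs the BT_Enemy behavior tree on possession.
; AI perception updates for TroopCharacters feed the blackboard, setting HasLineOfSight and EnemyActor when one is sensed.
; Losing a troop starts a LineOfSightTimer delay that clears both keys on expiry, and a new sighting cancels it, giving enemies a short memory of their target.
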(event OnTargetPerceptionUpdated(AIPerception)
  (params (Actor :type Actor%20Object%20Reference) (Stimulus :type AI%20Stimulus%20Structure))
  (bind _blackboard (Variables|Default|GetBlackboard))
  (bind _astroop_character (Utilities|Casting|CastToTroopCharacter Actor))
  (if (and (Utilities|IsValid _astroop_character) (.bSuccessfullySensed (Utilities|Struct|BreakAIStimulus Stimulus)))
    (Utilities|Time|ClearandInvalidateTimerbyHandle (Variables|Default|GetEnemy%20timer))
    (AI|Components|Blackboard|SetValueasBool _blackboard (Variables|Default|GetHasLineOfSight) true)
    (AI|Components|Blackboard|SetValueasObject _blackboard (Variables|Default|GetEnemyActor) _astroop_character)
    (else
      (bind _returnvalue (Utilities|Time|SetTimerbyEvent (delegate Custom|Start%20Enemy%20Timer) (Variables|Default|GetLine%20of%20sight%20timer)))
      (Variables|Default|SetEnemy%20timer _returnvalue))))

(event Custom|Start%20Enemy%20Timer
  (bind _blackboard (Variables|Default|GetBlackboard))
  (AI|Components|Blackboard|SetValueasBool _blackboard (Variables|Default|GetHasLineOfSight) false)
  (AI|Components|Blackboard|SetValueasObject _blackboard (Variables|Default|GetEnemyActor) 0))

(event EventPossess
  (params (PossessedPawn :type Pawn%20Object%20Reference))
  (AI|RunBehaviorTree "/Game/Characters/Enemy/AI/BT_Enemy.BT_Enemy"))

(fn ConstructionScript
  (|CallParentFunction))