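; AI controller for troop characters that starts their behavior tree when it possesses them.
; On possess, it reads the team tag from the troop's data asset and runs BT_Ally for allies or BT_Enemy for any other team.
; An unconnected chain that would write the castle and a random point in its forward attackable area to the blackboard never runs.
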(event EventPossess
  (params (PossessedPawn :type Pawn%20Object%20Reference))
  (bind _astroop_character (Utilities|Casting|CastToTroopCharacter PossessedPawn))
  (if (== (GameplayTags|GetTagName (Variables|/Script/MedievalDefense.TroopDataAsset|GetTeamTag (Variables|/Script/MedievalDefense.TroopCharacter|GetTroopDataAsset _astroop_character))) "Ally")
    (AI|RunBehaviorTree "/Game/Characters/Ally/AI/BT_Ally.BT_Ally")
    (else
      (AI|RunBehaviorTree "/Game/Characters/Enemy/AI/BT_Enemy.BT_Enemy"))))

(fn ConstructionScript)