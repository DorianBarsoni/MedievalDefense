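; BP_DeathNotify is an animation notify that finalizes a troop character's death.
; On firing, it casts the mesh owner to TroopCharacter and checks the team tag in its troop data asset.
; Troops tagged Enemy report the kill to the BP_GM_MedievalDefense game mode through EnemyKilled.
; The troop actor is then destroyed, though a failed game mode cast leaves an enemy in place.
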(fn ReceivedNotify
  (params (MeshComp :type Skeletal%20Mesh%20Component%20Object%20Reference) (Animation :type Anim%20Sequence%20Base%20Object%20Reference) (EventReference :type Anim%20Notify%20Event%20Reference%20Structure%20%28by%20ref%29))
  (bind _astroop_character (Utilities|Casting|CastToTroopCharacter (Components|GetOwner MeshComp)))
  (if (== "Enemy" (GameplayTags|GetTagName (Variables|/Script/MedievalDefense.TroopDataAsset|GetTeamTag (Variables|/Script/MedievalDefense.TroopCharacter|GetTroopDataAsset _astroop_character))))
    (bind _asbp_gm_medieval_defense (Utilities|Casting|CastToBP_GM_MedievalDefense (Game|GetGameMode)))
    (Class|GMMedievalDefense|EnemyKilled _asbp_gm_medieval_defense))
  (Actor|DestroyActor _astroop_character)
  (return true))