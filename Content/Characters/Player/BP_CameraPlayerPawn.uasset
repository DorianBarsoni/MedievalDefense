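; Player camera pawn that registers an Enhanced Input mapping context and smoothly switches its camera between two fixed angles.
; BeginPlay adds the mapping context to the owning player controller's input subsystem.
; The RotateCamera event plays or reverses a Timeline based on IsRotated, lerping the camera's relative rotation between the two angles.
; IsRotated is only read in this graph, never set.
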(event Custom|RotateCamera
  (if (Variables|Default|GetIsRotated)
    (bind _zerotoone (Timeline|Timeline Play)
      (:Update
        (Transformation|SetRelativeRotation (Variables|Default|GetCamera) (Math|Rotator|Lerp(Rotator) "-30.000000,0.000000,0.000000" "-60.000000,0.000000,0.000000" _zerotoone) false false)))
    (else
      (Timeline|Timeline Reverse))))

(event EventBeginPlay
  (bind _asplayer_controller (Utilities|Casting|CastToPlayerController (Pawn|GetController)))
  (Input|AddMappingContext (PlayerController|LocalPlayerSubsystems|GetEnhancedInputLocalPlayerSubsystem _asplayer_controller) "/Game/Characters/Player/InputMappingContext.InputMappingContext" 0 "(bIgnoreAllPressedKeysUntilRelease=True,bForceImmediately=False,bNotifyUserSettings=False)"))

(event Collision|EventActorBeginOverlap
  (params (OtherActor :type Actor%20Object%20Reference)))

(event EventTick
  (params (DeltaSeconds :type Float%20%28single-precision%29)))

(fn ConstructionScript)