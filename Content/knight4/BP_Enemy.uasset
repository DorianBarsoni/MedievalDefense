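; BP_Enemy is an enemy character that walks to the castle and repeatedly plays a sword slash once it arrives.
; On BeginPlay it runs AIMoveTo toward the first BP_Castle found, and success sets CanAttack.
; Tick uses CanAttack as a gate, playing the slash montage and delaying by its returned duration before re-arming.
; The graph only animates the attack and applies no damage.
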(event EventBeginPlay
  (bind _outactors (Actor|GetAllActorsOfClass "/Game/castle/BP_Castle.BP_Castle_C"))
  (AI|AIMoveTo self "0, 0, 0" (Utilities|Array|Get(acopy) _outactors) 7e+01 false
    (:OnSuccess
      (Variables|Default|SetcanAttack true))))

(event EventTick
  (params (DeltaSeconds :type Float%20%28single-precision%29))
  (if (Variables|Default|GetcanAttack)
    (Variables|Default|SetcanAttack false)
    (bind _returnvalue (Animation|PlayAnimMontage "/Game/knight4/Animations/Stable_Sword_Outward_Slash1_Montage.Stable_Sword_Outward_Slash1_Montage" 1.0 "None"))
    (Utilities|FlowControl|Delay _returnvalue)
    (Variables|Default|SetcanAttack true)))

(fn ConstructionScript)