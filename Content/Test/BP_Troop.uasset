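; BP_Troop is a test troop actor that is set up as an enemy and reports its team color on screen.
; Its construction script calls MakeTroopEnemy, whose body is defined outside this file.
; On BeginPlay, the custom PrintColor event prints the TeamComponent color as comma-separated RGBA for debugging.
; A second MakeTroopEnemy call in the event graph is unwired and never runs.
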(event Custom|Print%20Color
  (bind _teamcomponent (Variables|Default|GetTeamComponent))
  (bind _color (Variables|/Script/MedievalDefense.TeamComponent|GetColor _teamcomponent))
  (Development|PrintString (Utilities|String|Append (Utilities|String|ToString(Byte) (.r _color)) ", " (Utilities|String|ToString(Byte) (.g _color)) ", " (Utilities|String|ToString(Byte) (.b _color)) ", " (Utilities|String|ToString(Byte) (.a _color))) true true "(R=0.000000,G=0.660000,B=1.000000,A=1.000000)" 5.0))

(event EventBeginPlay
  (CallFunction|PrintColor))

(event Collision|EventActorBeginOverlap
  (params (OtherActor :type Actor%20Object%20Reference)))

(event EventTick
  (params (DeltaSeconds :type Float%20%28single-precision%29)))

(fn ConstructionScript
  (Class|TroopCharacter|MakeTroopEnemy))